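; Player actor with a Sphere component, moved by physics impulses or by dragging it with mouse or touch.
; MoveLeft, MoveRight, MoveUp and MoveDown push the sphere along X or Y, and Stop zeroes its velocity; none are called here.
; Click and touch toggle a gate meant to snap the actor to the cursor hit at constant height, but nothing enters it.
; An arrow-key polling chain is also disconnected.
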(event MouseInput|EventActorOnClicked
  (params (ButtonPressed :type Key%20Structure))
  (bind _returnvalue (Game|GetPlayerController 0))
  (bind _hitresult (Game|Player|GetHitResultUnderCursorbyChannel _returnvalue "TraceTypeQuery1" true))
  (bind _location (Collision|BreakHitResult _hitresult))
  (bind (_x _y) (Math|Vector|BreakVector _location))
  (Utilities|FlowControl|Gate true ; enters at Open
    (:Exit
      ;[1 1 1] Comment
      (Transformation|SetActorLocation (Math|Vector|MakeVector _x _y (.Z (Math|Vector|BreakVector (Transformation|GetActorLocation)))) false false))))

(event EventActorOnInputTouchBegin
  (params (FingerIndex :type ETouchIndex%20Enum :default "Touch1"))
  (bind _returnvalue (Game|GetPlayerController 0))
  (bind _hitresult (Game|Player|GetHitResultUnderCursorbyChannel _returnvalue "TraceTypeQuery1" true))
  (bind _location (Collision|BreakHitResult _hitresult))
  (bind (_x _y) (Math|Vector|BreakVector _location))
  (Utilities|FlowControl|Gate true ; enters at Open
    (:Exit
      ;[1 1 1] Comment
      (Transformation|SetActorLocation (Math|Vector|MakeVector _x _y (.Z (Math|Vector|BreakVector (Transformation|GetActorLocation)))) false false))))

(event EventActorOnReleased
  (params (ButtonReleased :type Key%20Structure))
  (bind _returnvalue (Game|GetPlayerController 0))
  (bind _hitresult (Game|Player|GetHitResultUnderCursorbyChannel _returnvalue "TraceTypeQuery1" true))
  (bind _location (Collision|BreakHitResult _hitresult))
  (bind (_x _y) (Math|Vector|BreakVector _location))
  (Utilities|FlowControl|Gate true ; enters at Close
    (:Exit
      ;[1 1 1] Comment
      (Transformation|SetActorLocation (Math|Vector|MakeVector _x _y (.Z (Math|Vector|BreakVector (Transformation|GetActorLocation)))) false false))))

(event EventActorOnInputTouchEnd
  (params (FingerIndex :type ETouchIndex%20Enum :default "Touch1"))
  (bind _returnvalue (Game|GetPlayerController 0))
  (bind _hitresult (Game|Player|GetHitResultUnderCursorbyChannel _returnvalue "TraceTypeQuery1" true))
  (bind _location (Collision|BreakHitResult _hitresult))
  (bind (_x _y) (Math|Vector|BreakVector _location))
  (Utilities|FlowControl|Gate true ; enters at Close
    (:Exit
      ;[1 1 1] Comment
      (Transformation|SetActorLocation (Math|Vector|MakeVector _x _y (.Z (Math|Vector|BreakVector (Transformation|GetActorLocation)))) false false))))

(fn ConstructionScript)

(fn MoveLeft
  (Physics|AddImpulse (Variables|Default|GetSphere) (Math|Vector|MakeVector 0.0 (Variables|Default|GetNegImpulse) 0.0) "None" false))

(fn MoveRight
  (Physics|AddImpulse (Variables|Default|GetSphere) (Math|Vector|MakeVector 0.0 (Variables|Default|GetImpulse) 0.0) "None" false))

(fn MoveUp
  (Physics|AddImpulse (Variables|Default|GetSphere) (Math|Vector|MakeVector (Variables|Default|GetImpulse) 0.0 0.0) "None" false))

(fn MoveDown
  (Physics|AddImpulse (Variables|Default|GetSphere) (Math|Vector|MakeVector (Variables|Default|GetNegImpulse) 0.0 0.0) "None" false))

(fn Stop
  (Class|PrimitiveComponent|SetAllPhysicsLinearVelocity (Variables|Default|GetSphere) "0, 0, 0" false))