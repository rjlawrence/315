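; BP_Maze procedurally builds a random grid maze in its construction script, reseeding on each run, with optional border and maze.
; An iterative depth-first carver steps two tiles in random directions, recording linking "bridge" tiles.
; At dead ends it backtracks to an unchecked path tile and converts the last bridge to path until none remain.
; Unused cells become walls, and instanced meshes render border, walls and floor from flat grid indices.
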(event EventBeginPlay)

(event Collision|EventActorBeginOverlap
  (params (OtherActor :type Actor%20Object%20Reference)))

(event EventTick
  (params (DeltaSeconds :type Float%20%28single-precision%29)))

(fn ConstructionScript
  (Math|Random|SetRandomStreamSeed (Variables|Default|GetRandom%20Stream) (Math|Random|RandomInteger 1000))
  (CallFunction|PopulateBoarder (Variables|Default|GetSize) (Variables|Default|GetBorder%20Tiles))
  (if (Variables|Default|GetShow%20Boarder?)
    (Utilities|SpawnInstances (Variables|Default|GetBorder%20Tiles) (Variables|Default|GetSize) (Variables|Default|GetTile%20Size) "1.000000,1.000000,1.000000" (Variables|Default|GetWall)
      (:Finished
        _)))
  (if (Variables|Default|GetShow%20Maze?)
    (CallFunction|SetInitialTile)
    (while (Variables|Default|GetCurrent%20Side%20Free?) :!label _label
      (CallFunction|PickNearbyTile))
    (Utilities|Array|Add (Variables|Default|GetChecked%20Tiles) (Variables|Default|GetCurrent%20Tile))
    (CallFunction|BackTrack)
    (Utilities|ConvertLastBridge
      (:Bridges%20Left
        (goto _label))
      (:No%20Bridges%20Left
        (CallFunction|PopulateWalls)
        (Utilities|SpawnInstances (Variables|Default|GetWall%20Tiles) (Variables|Default|GetSize) (Variables|Default|GetTile%20Size) "1.000000,1.000000,1.000000" (Variables|Default|GetBoxes)
          (:Finished
            (Utilities|SpawnInstances (Variables|Default|GetPath%20Tiles) (Variables|Default|GetSize) (Variables|Default|GetTile%20Size) "1.000000,1.000000,1.000000" (Variables|Default|GetFloor)
              (:Finished
                (Rendering|Material|SetMaterial (Variables|Default|GetFloor) 0 "/Game/StarterContent/Materials/M_Brick_Hewn_Stone.M_Brick_Hewn_Stone")))))))))

(fn PopulateBoarder
  (params (Size :type Integer) (Boarder%20Array :type Array%20of%20Integers))
  (LocalVariables|SetL_Size Size)
  ;[1 1 1] North
  (for _index (range 0 (- (LocalVariables|GetL_Size) 1))
    (Utilities|Array|Add Boarder%20Array _index))
  ;[1 1 1] East
  (for _index_2 (range 0 (- (LocalVariables|GetL_Size) 2))
    (Utilities|Array|Add Boarder%20Array (+ (* _index_2 (LocalVariables|GetL_Size)) (- (LocalVariables|GetL_Size) 1))))
  ;[1 1 1] South
  (for _index_3 (range 0 (LocalVariables|GetL_Size))
    (Utilities|Array|Add Boarder%20Array (+ (- _index_3 1) (* (LocalVariables|GetL_Size) (- (LocalVariables|GetL_Size) 1)))))
  ;[1 1 1] West
  (for _index_4 (range 0 (- (LocalVariables|GetL_Size) 2))
    (Utilities|Array|Add Boarder%20Array (* _index_4 (LocalVariables|GetL_Size)))))

(fn SetInitialTile
  (Variables|Default|SetCurrent%20Tile (+ (Variables|Default|GetSize) 1))
  (Utilities|Array|Add (Variables|Default|GetPath%20Tiles) (Variables|Default|GetCurrent%20Tile)))

(fn AddBridge&PathTile
  (params (Path%20Tile :type Integer) (Bridge%20Tile :type Integer))
  (Utilities|Array|Add (Variables|Default|GetPath%20Tiles) Path%20Tile)
  (Variables|Default|SetCurrent%20Tile Path%20Tile)
  (Utilities|Array|Add (Variables|Default|GetBridge%20Tiles) Bridge%20Tile))

(fn PickNearbyTile
  (bind _current_tile (Variables|Default|GetCurrent%20Tile))
  (bind _current_tile_2 (Variables|Default|GetCurrent%20Tile))
  (bind _size (Variables|Default|GetSize))
  (bind _current_tile_3 (Variables|Default|GetCurrent%20Tile))
  (bind _size_2 (Variables|Default|GetSize))
  (bind _current_tile_4 (Variables|Default|GetCurrent%20Tile))
  (bind (_tile_in_array_ _path_tile _bridge_tile) (Utilities|CheckEastTile _current_tile_2 false))
  (bind (_tile_in_arrays_ _path_tile_2 _bridge_tile_2) (Utilities|CheckNorthTile _current_tile_3 _size true))
  (bind (_tile_in_array__2 _path_tile_3 _bridge_tile_3) (Utilities|CheckEastTile _current_tile true))
  (bind (_tile_in_arrays__2 _path_tile_4 _bridge_tile_4) (Utilities|CheckNorthTile _current_tile_4 _size_2 false))
  (switch int (Math|Random|RandomIntegerinRangefromStream 0 3 (Variables|Default|GetRandom%20Stream))
    (:0
      (if _tile_in_arrays__2 :!label _label
        (Utilities|Counter (LocalVariables|GetCycleCounter) 4
          (:True
            (if _tile_in_arrays_ :!label _label_2
              (Utilities|Counter (LocalVariables|GetCycleCounter) 4
                (:True
                  (if _tile_in_array_ :!label _label_3
                    (Utilities|Counter (LocalVariables|GetCycleCounter) 4
                      (:True
                        (if _tile_in_array__2 :!label _label_4
                          (Utilities|Counter (LocalVariables|GetCycleCounter) 4
                            (:True
                              (goto _label))
                            (:False
                              (Variables|Default|SetCurrent%20Side%20Free? false :!label _label_5)))
                          (else
                            (CallFunction|AddBridge&PathTile _path_tile_3 _bridge_tile_3))))
                      (:False
                        (goto _label_5)))
                    (else
                      (CallFunction|AddBridge&PathTile _path_tile _bridge_tile))))
                (:False
                  (goto _label_5)))
              (else
                (CallFunction|AddBridge&PathTile _path_tile_2 _bridge_tile_2))))
          (:False
            (goto _label_5)))
        (else
          (CallFunction|AddBridge&PathTile _path_tile_4 _bridge_tile_4))))
    (:1
      (goto _label_3))
    (:2
      (goto _label_2))
    (:3
      (goto _label_4)))
  (return))

(fn BackTrack
  (bind _array_element (Utilities|ReverseforEachwithBreak (Variables|Default|GetPath%20Tiles) :!label _label)
    (:Loop%20Body
      (if (not (Utilities|Array|ContainsItem (Variables|Default|GetChecked%20Tiles) _array_element))
        (Variables|Default|SetCurrent%20Tile _array_element)
        (goto _label Break)))))

(fn PopulateWalls
  (bind _size (Variables|Default|GetSize))
  (for _index (range 0 (- (* _size _size) 1))
    (if (not (Utilities|CheckTileArray _index))
      (Utilities|Array|Add (Variables|Default|GetWall%20Tiles) _index))))